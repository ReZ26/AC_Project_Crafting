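; Inventory component that handles item pickup, the inventory screen and crafting support for its owning character.
; Pickup sphere-traces from the follow camera, stacks items in a name-keyed map and destroys the picked actor.
; The inventory key toggles a lazily created widget, switching input mode and mapping contexts, while crafting functions check, remove and add items.
; A similar trace feeds HUD item info, but its looping timer is unconnected here.
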(event Custom|Start%20Display%20Item%20Info
  (bind _owningactor (Variables|Default|GetOwningActor))
  (bind _hud_ui (Variables|Default|GetHud%20UI))
  (bind _followcamera (Variables|/Game/ThirdPerson/Blueprints/BP_ThirdPersonCharacter.BP_ThirdPersonCharacter_C|GetFollowCamera _owningactor))
  (bind _returnvalue (Transformation|GetWorldLocation _followcamera))
  (bind (_outhit _returnvalue_2) (Collision|SphereTraceForObjects _returnvalue (+ _returnvalue (* (Math|Vector|GetForwardVector _followcamera) (+ (Variables|/Script/Engine.SpringArmComponent|GetTargetArmLength (Variables|/Game/ThirdPerson/Blueprints/BP_ThirdPersonCharacter.BP_ThirdPersonCharacter_C|GetCameraBoom _owningactor)) 5e+02))) 1e+01 (Utilities|Array|MakeArray "ObjectTypeQuery1") false 0 "None"))
  (if _returnvalue_2
    (bind _asa_item_pickup_base (Utilities|Casting|CastToA_ItemPickup_Base (.HitActor (Collision|BreakHitResult _outhit)))
      (:then
        (Default|ShowItemInfo _hud_ui)
        (Default|UpdateItemData _hud_ui (Default|GetItemData _asa_item_pickup_base))
        (Variables|/Game/Items/Widget/Inventory/WBP_Hud.WBP_Hud_C|SetActor%20World%20To%20Screen _hud_ui (Class|SlateBlueprintLibrary|ScreentoViewport (.ScreenPosition (Class|GameplayStatics|ProjectWorldtoScreen (Game|GetPlayerController 0) (Transformation|GetWorldLocation (Variables|/Game/Items/A_ItemPickup_Base.A_ItemPickup_Base_C|GetStaticMesh _asa_item_pickup_base)) false)))))
      (:CastFailed
        (Default|HideItemInfo _hud_ui :!label _label)))
    (else
      (goto _label))))

(event Input|EnhancedActionEvents|EnhancedInputActionIA_PickUp
  (params (ActionValue :type Boolean) (ElapsedSeconds :type Float%20%28double-precision%29) (TriggeredSeconds :type Float%20%28double-precision%29) (InputAction :type Input%20Action%20Object%20Reference :default "/Game/ThirdPerson/Input/Actions/IA_PickUp.IA_PickUp"))
  (bind _owningactor (Variables|Default|GetOwningActor))
  (bind _followcamera (Variables|/Game/ThirdPerson/Blueprints/BP_ThirdPersonCharacter.BP_ThirdPersonCharacter_C|GetFollowCamera _owningactor))
  (bind _returnvalue (Transformation|GetWorldLocation _followcamera))
  (:Completed
    (bind _inventoryui (Variables|Default|GetInventoryUI)
      (:then
        (if (not (Widget|IsVisible _inventoryui))
          (bind (_outhit _returnvalue_2) (Collision|SphereTraceByChannel _returnvalue (+ _returnvalue (* (Math|Vector|GetForwardVector _followcamera) (+ (Variables|/Script/Engine.SpringArmComponent|GetTargetArmLength (Variables|/Game/ThirdPerson/Blueprints/BP_ThirdPersonCharacter.BP_ThirdPersonCharacter_C|GetCameraBoom _owningactor)) 5e+02))) 1e+01 "TraceTypeQuery1" false 0 "ForDuration" :!label _label))
          (if _returnvalue_2
            (bind _added_ (CallFunction|TryAddItem (.HitActor (Collision|BreakHitResult _outhit))))
            (if _added_
              (Actor|DestroyActor (.HitActor (Collision|BreakHitResult _outhit)))))))
      (:else
        (goto _label)))))

(event Input|EnhancedActionEvents|EnhancedInputActionIA_Inventory
  (params (ActionValue :type Boolean) (ElapsedSeconds :type Float%20%28double-precision%29) (TriggeredSeconds :type Float%20%28double-precision%29) (InputAction :type Input%20Action%20Object%20Reference :default "/Game/ThirdPerson/Input/Actions/IA_Inventory.IA_Inventory"))
  (bind _returnvalue (Game|GetPlayerController 0))
  (bind _returnvalue_2 (Game|GetPlayerController 0))
  (:Completed
    (Utilities|IsValid (Variables|Default|GetInventoryUI)
      (:Is%20Valid
        (if (Widget|IsVisible (Variables|Default|GetInventoryUI))
          (Widget|SetVisibility (Variables|Default|GetInventoryUI) "Hidden")
          (Input|SetInputModeGameOnly _returnvalue false)
          (Variables|/Script/Engine.PlayerController|SetbShowMouseCursor _returnvalue false)
          (bind _asmy_player_controller (Utilities|Casting|CastToMyPlayerController (Game|GetPlayerController 0)))
          (Default|AddMappingContext _asmy_player_controller "/Game/ThirdPerson/Input/IMC_Default.IMC_Default")
          (Default|AddMappingContext _asmy_player_controller "/Game/ThirdPerson/Input/IMC_Crafting.IMC_Crafting")
          (else
            (UserInterface|Viewport|AddtoViewport (stale _output_get) 0 :!label _label)
            (Input|SetInputModeGameandUI _returnvalue_2 (Variables|Default|GetInventoryUI) "DoNotLock" true false)
            (Variables|/Script/Engine.PlayerController|SetbShowMouseCursor _returnvalue_2 true)
            (Widget|SetVisibility (Variables|Default|GetInventoryUI) "Visible")
            (bind _asmy_player_controller_2 (Utilities|Casting|CastToMyPlayerController (Game|GetPlayerController 0)))
            (Default|RemoveMappingContext _asmy_player_controller_2 "/Game/ThirdPerson/Input/IMC_Default.IMC_Default")
            (Default|RemoveMappingContext _asmy_player_controller_2 "/Game/ThirdPerson/Input/IMC_Crafting.IMC_Crafting")
            (Default|UpdateInventory (Variables|Default|GetInventoryUI) (Variables|Default|GetInventory)))))
      (:Is%20Not%20Valid
        (bind _returnvalue_3 (Game|ConstructObjectfromClass "/Game/Items/Widget/Inventory/WBP_Inventory.WBP_Inventory_C"))
        (bind _output_get (Variables|Default|SetInventoryUI _returnvalue_3))
        (goto _label)))))

(event EventBeginPlay
  (bind _returnvalue (Game|ConstructObjectfromClass "/Game/Items/Widget/Inventory/WBP_Hud.WBP_Hud_C"))
  (Variables|Default|SetHud%20UI _returnvalue)
  (UserInterface|Viewport|AddtoViewport _returnvalue 0))

(event EventTick
  (params (DeltaSeconds :type Float%20%28single-precision%29)))

(fn TryAddItem
  (params (Hit%20Actor :type Actor%20Object%20Reference))
  (bind _asa_item_pickup_base (Utilities|Casting|CastToA_ItemPickup_Base Hit%20Actor)
    (:then
      (bind _output_get (LocalVariables|SetCurrentItem (Default|GetItemData _asa_item_pickup_base)))
      (if (CallFunction|IsItemAlreadyinInventory _output_get)
        (CallFunction|IncreaseItemAmount (LocalVariables|GetCurrentItem))
        (else
          (CallFunction|AddItemtoInventory (LocalVariables|GetCurrentItem))))
      (Development|PrintString (Utilities|String|Append (.Name (Utilities|Struct|BreakS_ItemData (LocalVariables|GetCurrentItem))) "Added"))
      (return true))
    (:CastFailed
      (LocalVariables|SetCurrentItem "")
      (return false))))

(fn IsItemAlreadyinInventory
  (params (Item :type S%20Item%20Data%20Structure))
  (return (Utilities|Map|Contains (Variables|Default|GetInventory) (.Name (Utilities|Struct|BreakS_ItemData Item)))))

(fn AddItemtoInventory
  (params (Item :type S%20Item%20Data%20Structure))
  (Utilities|Map|Add (Variables|Default|GetInventory) (.Name (Utilities|Struct|BreakS_ItemData Item)) Item))

(fn IncreaseItemAmount
  (params (Item :type S%20Item%20Data%20Structure))
  (LocalVariables|SetItem%20Name (.Name (Utilities|Struct|BreakS_ItemData Item)))
  (bind _result (Math|Integer|IncrementInt (.Amount (Utilities|Struct|BreakS_ItemData (.Value (Utilities|Map|Find (Variables|Default|GetInventory) (LocalVariables|GetItem%20Name))))))
    (:%20%20
      (bind _structout (Utilities|Struct|SetmembersinS_ItemData (.Value (Utilities|Map|Find (Variables|Default|GetInventory) (LocalVariables|GetItem%20Name))) _result))
      (Utilities|Map|Add (Variables|Default|GetInventory) (LocalVariables|GetItem%20Name) _structout))))

(fn GetItemAmountfromInventory
  (params (item%20Name :type String))
  (return (.Amount (Utilities|Struct|BreakS_ItemData (.Value (Utilities|Map|Find (Variables|Default|GetInventory) item%20Name))))))

(fn IsIteminInventory
  (params (Name :type String))
  (bind _inventory (Variables|Default|GetInventory))
  (bind (_value _returnvalue) (Utilities|Map|Find _inventory Name))
  (return _value _returnvalue))

(fn CanCraft
  (params (ingredients :type Map%20of%20A%20Item%20Pickup%20Base%20Soft%20Class%20References%20to%20Integers))
  (bind _keys (Utilities|Map|Keys ingredients))
  (for _array_element _keys
    (if (.ReturnValue (Utilities|Map|Find (Variables|Default|GetInventory) (Utilities|GetClassDefaults (Utilities|ResolveSoftReference _array_element))))
      (if (not (>= (Utilities|Struct|BreakS_ItemData (.Value (Utilities|Map|Find (Variables|Default|GetInventory) (Utilities|GetClassDefaults (Utilities|ResolveSoftReference _array_element))))) (.Value (Utilities|Map|Find ingredients _array_element))))
        (return false))
      (else
        (return false))))
  (return true))

(fn CraftItem
  (params (Crafting%20Item :type A%20Item%20Pickup%20Base%20Soft%20Class%20Reference))
  (bind _output (Utilities|ResolveSoftReference Crafting%20Item))
  (bind (_name _weight _cartgory _description _value) (Utilities|GetClassDefaults _output))
  (bind _s_itemdata (Utilities|Struct|MakeS_ItemData _name _weight _value _description _cartgory 1))
  (bind _has_item_ (CallFunction|IsIteminInventory _name))
  (if _has_item_
    (CallFunction|IncreaseItemAmount _s_itemdata)
    (else
      (CallFunction|AddItemtoInventory _s_itemdata))))

(fn RemoveIngredients
  (params (Remove%20Ingredients :type Map%20of%20A%20Item%20Pickup%20Base%20Soft%20Class%20References%20to%20Integers))
  (bind _keys (Utilities|Map|Keys Remove%20Ingredients))
  (for _array_element _keys
    (CallFunction|RemoveItembyAmount (.Name (Utilities|GetClassDefaults (Utilities|ResolveSoftReference _array_element))) (.Value (Utilities|Map|Find Remove%20Ingredients _array_element)))))

(fn RemoveItembyAmount
  (params (Item%20Name :type String%20%28by%20ref%29) (Amount :type Integer))
  (bind _inventory (Variables|Default|GetInventory))
  (bind _inventory_2 (Variables|Default|GetInventory))
  (bind _value (Utilities|Map|Find _inventory_2 Item%20Name))
  (bind (_value_2 _returnvalue) (Utilities|Map|Find _inventory Item%20Name))
  (if _returnvalue
    (LocalVariables|SetFound%20Item _value_2)
    (for _index (range 0 (- Amount 1))
      (bind _structout (Utilities|Struct|SetmembersinS_ItemData (LocalVariables|GetFound%20Item) (- (Utilities|Struct|BreakS_ItemData _value_2) 1)))
      (Utilities|Map|Add (Variables|Default|GetInventory) Item%20Name _structout))
    (if (== (Utilities|Struct|BreakS_ItemData _value) 0)
      (Utilities|Map|Remove (Variables|Default|GetInventory) Item%20Name)
      (return "")
      (else
        (return _value)))))