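; AC_Crafting is a component that opens and closes the crafting menu from the IA_Crafting input action.
; It creates WBP_CraftingMenu on first use, keeps the reference, then toggles the widget's visibility on later presses.
; Opening switches to Game and UI input with a cursor and removes IMC_Default through MyPlayerController.
; Closing restores game-only input, hides the cursor and re-adds that mapping context.
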(event Input|EnhancedActionEvents|EnhancedInputActionIA_Crafting
  (params (ActionValue :type Boolean) (ElapsedSeconds :type Float%20%28double-precision%29) (TriggeredSeconds :type Float%20%28double-precision%29) (InputAction :type Input%20Action%20Object%20Reference :default "/Game/ThirdPerson/Input/Actions/IA_Crafting.IA_Crafting"))
  (bind _returnvalue (Game|GetPlayerController 0))
  (bind _returnvalue_2 (Game|GetPlayerController 0))
  (:Completed
    (Utilities|IsValid (Variables|Default|GetCraftingMenuUI)
      (:Is%20Valid
        (if (Widget|IsVisible (Variables|Default|GetCraftingMenuUI))
          (Widget|SetVisibility (Variables|Default|GetCraftingMenuUI) "Hidden")
          (Input|SetInputModeGameOnly _returnvalue false)
          (Variables|/Script/Engine.PlayerController|SetbShowMouseCursor _returnvalue false)
          (bind _asmy_player_controller (Utilities|Casting|CastToMyPlayerController (Game|GetPlayerController 0)))
          (Default|AddMappingContext _asmy_player_controller "/Game/ThirdPerson/Input/IMC_Default.IMC_Default")
          (else
            (UserInterface|Viewport|AddtoViewport (stale _output_get) 0 :!label _label)
            (Input|SetInputModeGameandUI _returnvalue_2 (Variables|Default|GetCraftingMenuUI) "DoNotLock" true false)
            (Variables|/Script/Engine.PlayerController|SetbShowMouseCursor _returnvalue_2 true)
            (Widget|SetVisibility (Variables|Default|GetCraftingMenuUI) "Visible")
            (bind _asmy_player_controller_2 (Utilities|Casting|CastToMyPlayerController (Game|GetPlayerController 0)))
            (Default|RemoveMappingContext _asmy_player_controller_2 "/Game/ThirdPerson/Input/IMC_Default.IMC_Default"))))
      (:Is%20Not%20Valid
        (bind _returnvalue_3 (Game|ConstructObjectfromClass "/Game/Items/Widget/WBP_CraftingMenu.WBP_CraftingMenu_C"))
        (bind _output_get (Variables|Default|SetCraftingMenuUI _returnvalue_3))
        (goto _label)))))

(event EventBeginPlay)

(event EventTick
  (params (DeltaSeconds :type Float%20%28single-precision%29)))