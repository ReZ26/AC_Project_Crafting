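; Actor component that stands in for a timeline, playing a float curve over a given duration.
; Start sets a one-shot timer for the duration and a fast looping update timer, capped at once per frame.
; Each update samples the curve at the one-shot timer's elapsed time, prints the value and broadcasts it through OnUpdate.
; When time runs out, it clears the update timer and calls OnFinished.
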(event Custom|Finished
  (Utilities|Time|ClearandInvalidateTimerbyHandle (Variables|Default|GetTimer))
  (Default|CallOnFinished))

(event Custom|Update
  (Development|PrintString (Utilities|String|ToString(Float) (Class|KismetMathLibrary|GetRuntimeFloatCurveValue (Variables|Default|GetCurve) (Class|KismetSystemLibrary|GetTimerElapsedTimeHandle (stale Custom|Start _returnvalue)) 0.0)))
  (Default|CallOnUpdate (Class|KismetMathLibrary|GetRuntimeFloatCurveValue (Variables|Default|GetCurve) (Class|KismetSystemLibrary|GetTimerElapsedTimeHandle (stale Custom|Start _returnvalue)) 0.0)))

(event Custom|Start
  (params (Time :type Float%20%28single-precision%29))
  (bind _returnvalue (Utilities|Time|SetTimerbyEvent (delegate Custom|Finished) Time))
  (bind _returnvalue_2 (Utilities|Time|SetTimerbyEvent (delegate Custom|Update) 0.01 true true))
  (Variables|Default|SetTimer _returnvalue_2))

(event EventTick
  (params (DeltaSeconds :type Float%20%28single-precision%29)))